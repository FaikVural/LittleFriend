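; BP_KutuluController is an AI controller for the Kutulu character, driving it through a behavior tree.
; On BeginPlay it calls the parent and runs BT_Kutulu, leaving decision logic to that tree.
; An unconnected leftover chain would set the blackboard's TargetObject to the third-person character and assign an enemy general state, but it never runs.
; Tick is disabled and the construction script only calls its parent.
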(event EventBeginPlay
  (|CallParentFunction)
  (AI|RunBehaviorTree "/Game/_LittleFriend/AI/Behaviour/BT/BT_Kutulu.BT_Kutulu"))

(event EventTick
  (params (DeltaSeconds :type Float%20%28single-precision%29))
  (|CallParentFunction DeltaSeconds) ; This node is disabled and will not be called.\nDrag off pins to build functionality.
)

(fn ConstructionScript
  (|CallParentFunction))