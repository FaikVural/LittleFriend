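; Base AI controller that drives enemy reactions to seeing or hearing BP_LittleFriend through AI Perception and the Blackboard.
; Perception updates are sorted by sense into sight and hearing handlers, which change the enemy state and write TargetObject, plus TargetLocation for hearing.
; Losing sight reuses the sight handler with an empty target, so the same state is set.
; ChangeState saves the previous state as LastGeneralState before writing the new one.
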(event OnPerceptionUpdated(AIPerception)
  (params (UpdatedActors :type Array%20of%20Actor%20Object%20References))
  (Development|PrintString "ON PERCEPTION UPDATE")
  (for _array_element UpdatedActors
    (bind _asbp_little_friend (Utilities|Casting|CastToBP_LittleFriend _array_element))
    (bind _info (Class|AIPerceptionComponent|GetActorsPerception (Variables|Default|GetAIPerception) _asbp_little_friend))
    (for _array_element_2 (.LastSensedStimuli (Utilities|Struct|BreakActorPerceptionBlueprintInfo _info))
      (bind _returnvalue (Class|AIPerceptionSystem|GetSenseClassforStimulus _array_element_2))
      (Utilities|FlowControl|Sequence
        (:then_0
          (if (== _returnvalue "/Script/AIModule.AISense_Sight")
            (if (.bSuccessfullySensed (Utilities|Struct|BreakAIStimulus _array_element_2))
              (CallFunction|HandleSight _asbp_little_friend)
              (else
                (CallFunction|HandleSight)))))
        (:then_1
          (if (== _returnvalue "/Script/AIModule.AISense_Hearing")
            (if (.bSuccessfullySensed (Utilities|Struct|BreakAIStimulus _array_element_2))
              (Development|PrintString "hearrrrr")
              (CallFunction|HandleHearing (.StimulusLocation (Utilities|Struct|BreakAIStimulus _array_element_2)) _asbp_little_friend))))))))

(event EventBeginPlay)

(event EventTick
  (params (DeltaSeconds :type Float%20%28single-precision%29)))

(fn ConstructionScript)

(fn HandleSight
  (params (PerceivedActor :type Actor%20Object%20Reference))
  (CallFunction|ChangeState (Utilities|Enum|LiteralenumE_EnemyGeneralState "NewEnumerator1"))
  (AI|Components|Blackboard|SetValueasObject (AI|GetBlackboard 0) (Utilities|Name|MakeLiteralName "TargetObject") PerceivedActor))

(fn HandleHearing
  (params (HearingLocation :type Vector) (PerceivedActor :type Actor%20Object%20Reference))
  (bind _returnvalue (AI|GetBlackboard 0))
  (CallFunction|ChangeState (Utilities|Enum|LiteralenumE_EnemyGeneralState "NewEnumerator3"))
  (AI|Components|Blackboard|SetValueasVector _returnvalue (Utilities|Name|MakeLiteralName "TargetLocation") HearingLocation)
  (AI|Components|Blackboard|SetValueasObject _returnvalue (Utilities|Name|MakeLiteralName "TargetObject") PerceivedActor)
  (Development|PrintString "Hearing" true true "(R=1.000000,G=0.000000,B=0.114047,A=1.000000)"))

(fn ChangeState
  (params (NewState :type E_EnemyGeneralState%20Enum :default "NewEnumerator0"))
  (bind _returnvalue (AI|GetBlackboard 0))
  (AI|Components|Blackboard|SetValueasEnum _returnvalue (Utilities|Name|MakeLiteralName "LastGeneralState") (Class|BlackboardComponent|GetValueasEnum _returnvalue (Utilities|Name|MakeLiteralName "EnemyGeneralState")))
  (AI|Components|Blackboard|SetValueasEnum (AI|GetBlackboard 0) (Utilities|Name|MakeLiteralName "EnemyGeneralState") NewState))