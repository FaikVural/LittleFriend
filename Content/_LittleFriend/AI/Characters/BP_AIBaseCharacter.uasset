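; Base AI character that takes damage and ragdolls on death.
; Tick sets a ShouldMove flag from whether the movement velocity is non-zero.
; Health lives in the controller's Blackboard, and AnyDamage writes back the reduced value.
; The death check re-reads that updated value and subtracts Damage again, then Death switches the mesh to the Ragdoll collision profile with physics simulation.
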(event EventBeginPlay)

(event Collision|EventActorBeginOverlap
  (params (OtherActor :type Actor%20Object%20Reference)))

(event EventTick
  (params (DeltaSeconds :type Float%20%28single-precision%29))
  (if (> (Math|Vector|VectorLength (Variables|/Script/Engine.MovementComponent|GetVelocity (Variables|Character|GetCharacterMovement))) 0.0)
    (Variables|Default|SetShouldMove true)
    (else
      (Variables|Default|SetShouldMove false))))

(event Game|Damage|EventAnyDamage
  (params (Damage :type Float%20%28single-precision%29) (DamageType :type Damage%20Type%20Object%20Reference) (InstigatedBy :type Controller%20Object%20Reference) (DamageCauser :type Actor%20Object%20Reference))
  (bind _returnvalue (Pawn|GetController))
  (bind _returnvalue_2 (Utilities|Name|MakeLiteralName "Health"))
  (bind _returnvalue_3 (AI|GetBlackboard _returnvalue))
  (bind _returnvalue_4 (Class|BlackboardComponent|GetValueasFloat _returnvalue_3 _returnvalue_2))
  (bind _returnvalue_5 (- _returnvalue_4 Damage))
  (AI|Components|Blackboard|SetValueasFloat _returnvalue_3 _returnvalue_2 _returnvalue_5)
  (if (<= _returnvalue_5 0.0)
    (CallFunction|Death)))

(fn ConstructionScript)

(fn Death
  (bind _mesh (Variables|Character|GetMesh))
  (Development|PrintString "Death AI")
  (Collision|SetCollisionProfileName _mesh "Ragdoll" true :!class /Script/Engine.PrimitiveComponent)
  (Physics|SetSimulatePhysics _mesh true))