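; Sword weapon that gives its parent BP_LittleFriend a melee attack.
; Attack, gated by IsAttacking, immediately capsule-traces for Pawns just ahead of the mesh, ignoring the owner.
; A first hit switches mesh collision to Block and calls ApplyDamage, though no damaged actor is wired.
; It also plays a sped-up swing montage on the owner, whose completion clears the gate and restores Overlap collision.
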(event Custom|Attack
  (bind _staticmesh (Variables|Default|GetStaticMesh))
  (bind _returnvalue (Transformation|GetWorldLocation _staticmesh))
  (if (not (Variables|Default|GetIsAttacking))
    (Variables|Default|SetIsAttacking true)
    (bind _outhits (Class|KismetSystemLibrary|CapsuleTraceMultiforObjects _returnvalue (+ _returnvalue (* (Math|Vector|GetForwardVector _staticmesh) 2e+01)) 25.0 1e+01 (Utilities|Array|MakeArray "ObjectTypeQuery3") false (Utilities|Array|MakeArray (Variables|Default|GetLittleFriend)) "None" true "(R=1.000000,G=0.000000,B=0.000000,A=1.000000)" "(R=0.000000,G=1.000000,B=0.000000,A=1.000000)" 2.0))
    (Utilities|FlowControl|Sequence
      (:then_0
        (Utilities|Array|ForEachLoopwithBreak _outhits :!label _label
          (:LoopBody
            (Collision|SetCollisionResponsetoAllChannels _staticmesh "ECR_Block")
            (Game|Damage|ApplyDamage 0 5e+01 (Game|GetInstigatorController (Actor|GetParentActor)) self "/Script/Engine.DamageType")
            (goto _label Break))))
      (:then_1
        (Animation|Montage|PlayMontage (Variables|/Script/Engine.Character|GetMesh (Variables|Default|GetLittleFriend)) "/Game/_LittleFriend/Character/Animations/AM_StandingMeleeAttackHorizontalR.AM_StandingMeleeAttackHorizontalR" 2.0
          (:OnCompleted
            (Variables|Default|SetIsAttacking false)
            (Collision|SetCollisionResponsetoAllChannels _staticmesh "ECR_Overlap")))))))

(event EventBeginPlay
  (bind _asbp_little_friend (Utilities|Casting|CastToBP_LittleFriend (Actor|GetParentActor)))
  (Variables|Default|SetLittleFriend _asbp_little_friend))

(event Collision|EventActorBeginOverlap
  (params (OtherActor :type Actor%20Object%20Reference)))

(event EventTick
  (params (DeltaSeconds :type Float%20%28single-precision%29)))

(fn ConstructionScript)